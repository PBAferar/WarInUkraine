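; Trigger actor that marks where the player can perform a roof jump.
; Its box overlaps set and clear the KvJumpRoof flag on a BP_Kv_PlayerHand_Pawn tagged "Player".
; A Jump_Roof event, with no caller in this file, plays a timeline that sets the player character's root relative transform on each update, though no transform value is wired in.
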(event OnComponentBeginOverlap(Box)
  (params (OverlappedComponent :type Primitive%20Component%20Object%20Reference) (OtherActor :type Actor%20Object%20Reference) (OtherComp :type Primitive%20Component%20Object%20Reference) (OtherBodyIndex :type Integer) (bFromSweep :type Boolean) (SweepResult :type Hit%20Result%20Structure%20%28by%20ref%29))
  (if (Actor|ActorHasTag OtherActor "Player")
    (bind _asbp_kv_player_hand_pawn (Utilities|Casting|CastToBP_Kv_PlayerHand_Pawn OtherActor))
    (Variables|/Game/Kvik/Kvik_Modes/Players/Player_Hand/Test_hand/BP_Kv_PlayerHand_Pawn.BP_Kv_PlayerHand_Pawn_C|SetKv_Jump_Roof _asbp_kv_player_hand_pawn true)))

(event OnComponentEndOverlap(Box)
  (params (OverlappedComponent :type Primitive%20Component%20Object%20Reference) (OtherActor :type Actor%20Object%20Reference) (OtherComp :type Primitive%20Component%20Object%20Reference) (OtherBodyIndex :type Integer))
  (if (Actor|ActorHasTag OtherActor "Player")
    (bind _asbp_kv_player_hand_pawn (Utilities|Casting|CastToBP_Kv_PlayerHand_Pawn OtherActor))
    (Variables|/Game/Kvik/Kvik_Modes/Players/Player_Hand/Test_hand/BP_Kv_PlayerHand_Pawn.BP_Kv_PlayerHand_Pawn_C|SetKv_Jump_Roof _asbp_kv_player_hand_pawn false)))

(event Custom|Jump_Roof
  (Timeline|Timeline_0 PlayFromStart
    (:Update
      (Transformation|SetRelativeTransform (Variables|/Script/Engine.Actor|GetRootComponent (Game|GetPlayerCharacter 0)) (Math|Transform|MakeTransform (Math|Vector|MakeVector 0.0 0.0 0.0) "0, 0, 0" "1.000000,1.000000,1.000000") false false))))

(event EventBeginPlay)

(event Collision|EventActorBeginOverlap
  (params (OtherActor :type Actor%20Object%20Reference)))

(event EventTick
  (params (DeltaSeconds :type Float%20%28single-precision%29)))

(fn ConstructionScript)
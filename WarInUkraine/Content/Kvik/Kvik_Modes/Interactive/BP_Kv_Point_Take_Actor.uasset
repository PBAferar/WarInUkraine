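; BP_Kv_Point_Take_Actor is an interactive point actor for taking a Stugna weapon.
; Take_Stugna spawns a BP_Kv_Stagna_2_Ammo_Unistal_Pawn at the PointSpawnStugna transform, passes it KvCharged and calls ModeCharge.
; Take_Ammo_Stigna only checks ObjectAmmo and does nothing further.
; An ObjectStugna check leading to the same spawn is disconnected and never runs.
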(event Custom|Take_Ammo_Stigna
  (if (Variables|Default|GetObject_Ammo)
    _))

(event Custom|Take_Stugna
  (bind _returnvalue (Game|SpawnActorfromClass "/Game/Kvik/Kvik_Modes/Weapons/Stugna/BP_Kv_Stagna_2_Ammo_Unistal_Pawn.BP_Kv_Stagna_2_Ammo_Unistal_Pawn_C" (Transformation|GetWorldTransform (Variables|Default|GetPoint_Spawn_Stugna)) "Undefined" 0 0))
  (Variables|/Game/Kvik/Kvik_Modes/Weapons/Stugna/BP_Kv_Stagna_2_Ammo_Unistal_Pawn.BP_Kv_Stagna_2_Ammo_Unistal_Pawn_C|SetKv_Charged _returnvalue (Variables|Default|GetKv_charged))
  (Default|ModeCharge _returnvalue))

(event EventBeginPlay)

(event Collision|EventActorBeginOverlap
  (params (OtherActor :type Actor%20Object%20Reference)))

(fn ConstructionScript)
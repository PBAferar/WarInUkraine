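; BP_Kv_PlayerSit_Pawn is a Kvik player pawn, by its name for a seated player, that provides limited mouse look.
; Mouse turn input adds to the relative yaw of RotCamera, while inverted look-up input adds to the relative pitch of Camera.
; Both angles are clamped and the other axes are zeroed, splitting yaw and pitch across two components.
; The graphs contain no movement, tick or construction logic.
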(event EventBeginPlay)

(event Collision|EventActorBeginOverlap
  (params (OtherActor :type Actor%20Object%20Reference)))

(event EventTick
  (params (DeltaSeconds :type Float%20%28single-precision%29)))

(event Input|AxisEvents|InputAxisTurnRight/LeftMouse
  (params (AxisValue :type Float%20%28single-precision%29))
  (bind _rotcamera (Variables|Default|GetRotCamera))
  (Transformation|SetRelativeRotation _rotcamera (Math|Rotator|MakeRotator 0.0 0.0 (Math|Float|Clamp(Float) (+ (.yaw (Variables|/Script/Engine.SceneComponent|GetRelativeRotation _rotcamera)) AxisValue) -6e+01 6e+01)) false false))

(event Input|AxisEvents|InputAxisLookUp/DownMouse
  (params (AxisValue :type Float%20%28single-precision%29))
  (bind _camera (Variables|Default|GetCamera))
  (Transformation|SetRelativeRotation _camera (Math|Rotator|MakeRotator 0.0 (Math|Float|Clamp(Float) (+ (* AxisValue -1.0) (.pitch (Variables|/Script/Engine.SceneComponent|GetRelativeRotation _camera))) -6e+01 45.0) 0.0) false false))

(fn ConstructionScript)
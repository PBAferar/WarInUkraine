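; First-person player character with AK hands, handling mouse look, movement, Shift running, aiming, firing and reloading.
; Right mouse toggles aim animations while held or released, and Tick interpolates camera FOV for the zoom.
; Tick calls Fire_AK while left mouse is held; its Delay paces automatic shots that spawn an effect actor and play sound.
; Reload only plays hand and weapon animations plus sound, with no ammo logic.
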(event Custom|Fire_AK
  (bind _mesh (Variables|Character|GetMesh))
  ;[1 1 1] Выстрелы
  (Utilities|FlowControl|Delay 0.1)
  (if (Variables|Default|GetKv_Hand_Aim)
    (Components|Animation|PlayAnimation _mesh "/Game/Kvik/Kvik_Modes/Players/Player_Hand/Test_hand/kalashadsfire.kalashadsfire" false)
    (else
      (Components|Animation|PlayAnimation _mesh "/Game/Kvik/Kvik_Modes/Players/Player_Hand/Test_hand/kalashfire2_Fedir_1p_Anim.kalashfire2_Fedir_1p_Anim" false)))
  (Game|SpawnActorfromClass "/Game/Kvik/Effects/Blueprint_Effect_Shooting_AK.Blueprint_Effect_Shooting_AK_C" (Transformation|GetWorldTransform (Variables|Default|GetArrow1)) "Undefined" 0 0)
  (Audio|PlaySound2D "/Game/1WUI/Audio/ak.ak" 1.0 1.0 0.0 0 0))

(event Custom|Aim_AK
  (bind _mesh (Variables|Character|GetMesh))
  (if (Variables|Default|GetKv_Hand_Aim)
    (Components|Animation|PlayAnimation _mesh "/Game/Kvik/Kvik_Modes/Players/Player_Hand/Test_hand/kalashads.kalashads" false)
    (else
      (Components|Animation|PlayAnimation _mesh "/Game/Kvik/Kvik_Modes/Players/Player_Hand/Test_hand/kalashads_2.kalashads_2" false))))

(event EventBeginPlay)

(event Collision|EventActorBeginOverlap
  (params (OtherActor :type Actor%20Object%20Reference)))

(event EventTick
  (params (DeltaSeconds :type Float%20%28single-precision%29))
  (bind _camera (Variables|Camera|GetCamera))
  (if (Variables|Default|GetKv_Hand_Fire)
    (CallFunction|FireAK))
  (if (Variables|Default|GetKv_Hand_Aim)
    (bind _output_get (Variables|Default|SetKv_Field_Of_View (Math|Interpolation|FInterpTo (Variables|Default|GetKv_Field_Of_View) 4e+01 (Utilities|Time|GetWorldDeltaSeconds) 5.0)))
    (Camera|SetFieldOfView _camera _output_get)
    (else
      (bind _output_get_2 (Variables|Default|SetKv_Field_Of_View (Math|Interpolation|FInterpTo (Variables|Default|GetKv_Field_Of_View) 7e+01 (Utilities|Time|GetWorldDeltaSeconds) 5.0)))
      (Camera|SetFieldOfView _camera _output_get_2))))

(event Input|AxisEvents|InputAxisTurnRight/LeftMouse
  (params (AxisValue :type Float%20%28single-precision%29))
  ;[0.1539 1 0.1723] Камера
  (Pawn|Input|AddControllerYawInput AxisValue))

(event Input|AxisEvents|InputAxisLookUp/DownMouse
  (params (AxisValue :type Float%20%28single-precision%29))
  ;[0.1539 1 0.1723] Камера
  (Pawn|Input|AddControllerPitchInput AxisValue))

(event Input|AxisEvents|InputAxisMoveForward/Backward
  (params (AxisValue :type Float%20%28single-precision%29))
  ;[0.3473 1 0.2273] Двидение в перед, назад шаг в лево и в право
  (Pawn|Input|AddMovementInput (Transformation|GetActorForwardVector) AxisValue false))

(event Input|AxisEvents|InputAxisMoveRight/Left
  (params (AxisValue :type Float%20%28single-precision%29))
  ;[0.3473 1 0.2273] Двидение в перед, назад шаг в лево и в право
  (Pawn|Input|AddMovementInput (Transformation|GetActorRightVector) AxisValue false))

(event Input|KeyboardEvents|LeftShift
  (params (Key :type Key%20Structure :default "None"))
  (bind _charactermovement (Variables|Character|GetCharacterMovement))
  ;[0.08222 1 0.05575] Бег
  (:Pressed
    (Variables|/Script/Engine.CharacterMovementComponent|SetMaxWalkSpeed _charactermovement (+ (Variables|/Script/Engine.CharacterMovementComponent|GetMaxWalkSpeed _charactermovement) (Variables|Default|GetKv_Hand_SpeedRun))))
  (:Released
    (Variables|/Script/Engine.CharacterMovementComponent|SetMaxWalkSpeed _charactermovement (- (Variables|/Script/Engine.CharacterMovementComponent|GetMaxWalkSpeed _charactermovement) (Variables|Default|GetKv_Hand_SpeedRun)))))

(event Input|MouseEvents|LeftMouseButton
  (params (Key :type Key%20Structure :default "None"))
  (:Pressed
    (Variables|Default|SetKv_Hand_Fire true))
  (:Released
    (Variables|Default|SetKv_Hand_Fire false)))

(event Input|KeyboardEvents|R
  (params (Key :type Key%20Structure :default "None"))
  ;[1 1 1] Перзарядка
  (:Pressed
    (Components|Animation|PlayAnimation (Variables|Character|GetMesh) "/Game/Kvik/Kvik_Modes/Players/Player_Hand/Test_hand/kalashreload.kalashreload" false)
    (Components|Animation|PlayAnimation (Variables|Default|GetSkeletalMesh) "/Game/Kvik/Kvik_Modes/Players/Player_Hand/Test_hand/AK_Model/kalashreload_pasted__AK_model_Anim.kalashreload_pasted__AK_model_Anim" false)
    (Audio|PlaySound2D "/Game/1WUI/Audio/netoroplivaya-perezaryadka-ak-47.netoroplivaya-perezaryadka-ak-47" 1.0 1.2 0.0 0 0)))

(event Input|MouseEvents|RightMouseButton
  (params (Key :type Key%20Structure :default "None"))
  (:Pressed
    (Variables|Default|SetKv_Hand_Aim true)
    (CallFunction|AimAK :!label _label))
  (:Released
    (Variables|Default|SetKv_Hand_Aim false)
    (goto _label)))

(fn ConstructionScript)
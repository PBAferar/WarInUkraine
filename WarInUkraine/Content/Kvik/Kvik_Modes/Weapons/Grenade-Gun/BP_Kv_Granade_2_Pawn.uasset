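; Possessable grenade-gun pawn that the player aims with the mouse and fires to launch grenade projectiles.
; Yaw turns the Camera component, clamped pitch drives RotVertical, and left click spawns a grenade at PointBullet with a sound and a delay-based cooldown.
; E spawns and possesses a player hand pawn and repositions Zero.
; When Zero hits something, it stops simulating physics after a short delay and Basse moves to its location.
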(event OnComponentHit(zero)
  (params (HitComponent :type Primitive%20Component%20Object%20Reference) (OtherActor :type Actor%20Object%20Reference) (OtherComp :type Primitive%20Component%20Object%20Reference) (NormalImpulse :type Vector :default "0, 0, 0") (Hit :type Hit%20Result%20Structure%20%28by%20ref%29))
  (bind _zero (Variables|Default|Getzero))
  (Utilities|FlowControl|Delay 0.5)
  (Physics|SetSimulatePhysics _zero false)
  (Transformation|SetWorldLocation (Variables|Default|GetBasse) (Transformation|GetWorldLocation _zero) false false))

(event EventBeginPlay)

(event Collision|EventActorBeginOverlap
  (params (OtherActor :type Actor%20Object%20Reference)))

(event EventTick
  (params (DeltaSeconds :type Float%20%28single-precision%29)))

(event Input|AxisEvents|InputAxisTurnRight/LeftMouse
  (params (AxisValue :type Float%20%28single-precision%29))
  (Transformation|AddWorldRotation (Variables|Default|GetCamera) (Math|Rotator|MakeRotator 0.0 0.0 AxisValue) false false))

(event Input|AxisEvents|InputAxisLookUp/DownMouse
  (params (AxisValue :type Float%20%28single-precision%29))
  (bind _output_get (Variables|Default|SetSpeed (Math|Float|Clamp(Float) (+ AxisValue (Variables|Default|GetSpeed)) -3e+01 1e+01)))
  (Transformation|SetRelativeRotation (Variables|Default|GetRot_Vertical) (Math|Rotator|MakeRotator 0.0 _output_get 0.0) false false))

(event Input|MouseEvents|LeftMouseButton
  (params (Key :type Key%20Structure :default "None"))
  (:Pressed
    (if (not (Variables|Default|GetFire))
      (Variables|Default|SetFire true)
      (Game|SpawnActorfromClass "/Game/Kvik/Kvik_Modes/Weapons/Grenade-Gun/BP_Kv_Bullet_Grenad.BP_Kv_Bullet_Grenad_C" (Transformation|GetWorldTransform (Variables|Default|GetPointBullet)) "Undefined" 0 0)
      (Audio|PlaySound2D "/Game/1WUI/Audio/gluhoy-negromkiy-vyistrel.gluhoy-negromkiy-vyistrel" 1.0 1.0 0.0 0 0)
      (Utilities|FlowControl|Delay 3.0)
      (Variables|Default|SetFire false))))

(event Input|KeyboardEvents|E
  (params (Key :type Key%20Structure :default "None"))
  (bind _rot_vertical (Variables|Default|GetRot_Vertical))
  (bind _returnvalue (Transformation|GetSocketLocation _rot_vertical "None"))
  (:Pressed
    (bind _returnvalue_2 (Game|SpawnActorfromClass "/Game/Kvik/Kvik_Modes/Players/Player_Hand/Test_hand/BP_Kv_PlayerHand_Pawn.BP_Kv_PlayerHand_Pawn_C" (Transformation|GetWorldTransform (Variables|Default|GetSpawnPlayer)) "Undefined" 0 0))
    (Pawn|Possess (Game|GetPlayerController 0) _returnvalue_2)
    (Transformation|SetRelativeLocation (Variables|Default|Getzero) (Math|Vector|MakeVector (.x _returnvalue) (.y _returnvalue) (.z _returnvalue)) false false)))

(fn ConstructionScript)
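; Grenade-gun pawn in the Kvik weapon modes, with mouse look and an exit back to the player-hand pawn.
; Mouse X yaws the Sphere and mouse Y pitches the Arrow.
; Tick increments Speed and writes it as the Camera's world Z until a Sphere overlap sets Move, which halts this.
; E spawns BP_Kv_PlayerHand_Pawn at SpawnPlayer and possesses it, without destroying this pawn.
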(event OnComponentBeginOverlap(Sphere)
  (params (OverlappedComponent :type Primitive%20Component%20Object%20Reference) (OtherActor :type Actor%20Object%20Reference) (OtherComp :type Primitive%20Component%20Object%20Reference) (OtherBodyIndex :type Integer) (bFromSweep :type Boolean) (SweepResult :type Hit%20Result%20Structure%20%28by%20ref%29))
  (Variables|Default|SetMove true))

(event EventBeginPlay)

(event Collision|EventActorBeginOverlap
  (params (OtherActor :type Actor%20Object%20Reference)))

(event EventTick
  (params (DeltaSeconds :type Float%20%28single-precision%29))
  (if (not (Variables|Default|GetMove))
    (bind _result (Math|Float|IncrementFloat (Variables|Default|Getspeed))
      (:%20%20
        (bind _output_get (Variables|Default|Setspeed _result))
        (Transformation|SetWorldLocation (Variables|Default|GetCamera) (Math|Vector|MakeVector 0.0 0.0 _output_get) false false)))))

(event Input|AxisEvents|InputAxisTurnRight/LeftMouse
  (params (AxisValue :type Float%20%28single-precision%29))
  (Transformation|AddWorldRotation (Variables|Default|GetSphere) (Math|Rotator|MakeRotator 0.0 0.0 AxisValue) false false))

(event Input|AxisEvents|InputAxisLookUp/DownMouse
  (params (AxisValue :type Float%20%28single-precision%29))
  (Transformation|AddLocalRotation (Variables|Default|GetArrow) (Math|Rotator|MakeRotator 0.0 AxisValue 0.0) false false))

(event Input|MouseEvents|LeftMouseButton
  (params (Key :type Key%20Structure :default "None")))

(event Input|KeyboardEvents|E
  (params (Key :type Key%20Structure :default "None"))
  (:Pressed
    (bind _returnvalue (Game|SpawnActorfromClass "/Game/Kvik/Kvik_Modes/Players/Player_Hand/Test_hand/BP_Kv_PlayerHand_Pawn.BP_Kv_PlayerHand_Pawn_C" (Math|Transform|MakeTransform (Transformation|GetWorldLocation (Variables|Default|GetSpawnPlayer)) "0, 0, 0" "1.000000,1.000000,1.000000") "Undefined" 0 0))
    (Pawn|Possess (Game|GetPlayerController 0) _returnvalue)))

(fn ConstructionScript)
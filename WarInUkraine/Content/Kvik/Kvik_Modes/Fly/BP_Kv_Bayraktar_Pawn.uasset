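; Player-flown Bayraktar drone pawn that drops bombs and fires guided rockets, with mouse camera look and zoom.
; Tick drives constant forward flight with key-controlled yaw and altitude, and fades a material invisibility parameter by height.
; A camera line trace continually updates the target that launched rockets steer toward; bombs fall by physics, and both spawn explosions on hit.
; E possesses a new on-foot pawn and reloads saved ammo and health.
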(event OnComponentHit(Slot_Bomb_1)
  (params (HitComponent :type Primitive%20Component%20Object%20Reference) (OtherActor :type Actor%20Object%20Reference) (OtherComp :type Primitive%20Component%20Object%20Reference) (NormalImpulse :type Vector :default "0, 0, 0") (Hit :type Hit%20Result%20Structure%20%28by%20ref%29))
  ;[1 1 1] Взрыв бомб
  (if (not (Actor|ActorHasTag OtherActor "Bayraktar"))
    (Game|SpawnActorfromClass "/Game/Kvik/Effects/BP_Kv_ExplosionBig.BP_Kv_ExplosionBig_C" (Transformation|GetWorldTransform (Variables|Default|GetSlot_Bomb_1)) "Undefined" 0 0)
    (Components|DestroyComponent (Variables|Default|GetSlot_Bomb_1))))

(event OnComponentHit(Slot_Bomb_2)
  (params (HitComponent :type Primitive%20Component%20Object%20Reference) (OtherActor :type Actor%20Object%20Reference) (OtherComp :type Primitive%20Component%20Object%20Reference) (NormalImpulse :type Vector :default "0, 0, 0") (Hit :type Hit%20Result%20Structure%20%28by%20ref%29))
  ;[1 1 1] Взрыв бомб
  (if (not (Actor|ActorHasTag OtherActor "Bayraktar"))
    (Game|SpawnActorfromClass "/Game/Kvik/Effects/BP_Kv_ExplosionBig.BP_Kv_ExplosionBig_C" (Transformation|GetWorldTransform (Variables|Default|GetSlot_Bomb_2)) "Undefined" 0 0)
    (Components|DestroyComponent (Variables|Default|GetSlot_Bomb_2))))

(event OnComponentHit(Slot_Rocket_1)
  (params (HitComponent :type Primitive%20Component%20Object%20Reference) (OtherActor :type Actor%20Object%20Reference) (OtherComp :type Primitive%20Component%20Object%20Reference) (NormalImpulse :type Vector :default "0, 0, 0") (Hit :type Hit%20Result%20Structure%20%28by%20ref%29))
  ;[1 1 1] Взрыв бомб
  (if (not (Actor|ActorHasTag OtherActor "Bayraktar"))
    (Game|SpawnActorfromClass "/Game/Kvik/Effects/BP_Kv_ExplosionBig.BP_Kv_ExplosionBig_C" (Transformation|GetWorldTransform (Variables|Default|GetSlot_Rocket_1)) "Undefined" 0 0)
    (Variables|Default|SetRocket_1_Fire false)
    (Components|DestroyComponent (Variables|Default|GetSlot_Rocket_1))))

(event OnComponentHit(Slot_Rocket_2)
  (params (HitComponent :type Primitive%20Component%20Object%20Reference) (OtherActor :type Actor%20Object%20Reference) (OtherComp :type Primitive%20Component%20Object%20Reference) (NormalImpulse :type Vector :default "0, 0, 0") (Hit :type Hit%20Result%20Structure%20%28by%20ref%29))
  ;[1 1 1] Взрыв бомб
  (if (not (Actor|ActorHasTag OtherActor "Bayraktar"))
    (Game|SpawnActorfromClass "/Game/Kvik/Effects/BP_Kv_ExplosionBig.BP_Kv_ExplosionBig_C" (Transformation|GetWorldTransform (Variables|Default|GetSlot_Rocket_2)) "Undefined" 0 0)
    (Variables|Default|SetRocket_2_Fire false)
    (Components|DestroyComponent (Variables|Default|GetSlot_Rocket_2))))

(event Custom|Load_Ammo
  ;[0.2368 1 0.2457] загрузка данных
  (bind _returnvalue (SaveGame|LoadGamefromSlot "1"))
  (bind _ass_kv_save (Utilities|Casting|CastToS_Kv_Save _returnvalue))
  (bind _asbp_kv_player_hand_pawn (Utilities|Casting|CastToBP_Kv_PlayerHand_Pawn (Game|GetPlayerCharacter 0)))
  (Variables|/Game/Kvik/Kvik_Modes/Players/Player_Hand/Test_hand/BP_Kv_PlayerHand_Pawn.BP_Kv_PlayerHand_Pawn_C|SetKv_Ammo _asbp_kv_player_hand_pawn (Variables|/Game/Kvik/BP_Kv_Logik/S_Kv_Save.S_Kv_Save_C|GetS_Ammo_AK _ass_kv_save))
  (Variables|/Game/Kvik/Kvik_Modes/Players/Player_Hand/Test_hand/BP_Kv_PlayerHand_Pawn.BP_Kv_PlayerHand_Pawn_C|SetKv_All_Ammo _asbp_kv_player_hand_pawn (Variables|/Game/Kvik/BP_Kv_Logik/S_Kv_Save.S_Kv_Save_C|GetS_AllAmmo_AK _ass_kv_save))
  (Variables|/Game/Kvik/Kvik_Modes/Players/Player_Hand/Test_hand/BP_Kv_PlayerHand_Pawn.BP_Kv_PlayerHand_Pawn_C|SetKv_HP _asbp_kv_player_hand_pawn (Variables|/Game/Kvik/BP_Kv_Logik/S_Kv_Save.S_Kv_Save_C|GetS_HP_Player _ass_kv_save)))

(event Custom|FireRocket_1
  (if (Variables|Default|GetRocket_1_Fire)
    (Physics|SetSimulatePhysics (Variables|Default|GetSlot_Rocket_1) true)
    (Transformation|SetWorldRotation (Variables|Default|GetSlot_Rocket_1) (Math|Rotator|FindLookatRotation (Transformation|GetWorldLocation (Variables|Default|GetSlot_Rocket_1)) (Variables|Default|GetTarget_Rocket)) false false)
    (Class|SceneComponent|AddLocalTransform (Variables|Default|GetSlot_Rocket_1) (Math|Transform|MakeTransform "30.000000, 0, 0" "0, 0, 0" "1.000000,1.000000,1.000000") false false)))

(event Custom|Distance%20bomb
  ;[1 1 1] Время падения бомбы
  (Variables|Default|SetTime_Bomb (/ (.z (Transformation|GetActorLocation)) 2.81e+03)))

(event Custom|FireRocket_2
  (if (Variables|Default|GetRocket_2_Fire)
    (Physics|SetSimulatePhysics (Variables|Default|GetSlot_Rocket_2) true)
    (Transformation|SetWorldRotation (Variables|Default|GetSlot_Rocket_2) (Math|Rotator|FindLookatRotation (Transformation|GetWorldLocation (Variables|Default|GetSlot_Rocket_2)) (Variables|Default|GetTarget_Rocket)) false false)
    (Class|SceneComponent|AddLocalTransform (Variables|Default|GetSlot_Rocket_2) (Math|Transform|MakeTransform "30.000000, 0, 0" "0, 0, 0" "1.000000,1.000000,1.000000") false false)))

(event EventBeginPlay)

(event Collision|EventActorBeginOverlap
  (params (OtherActor :type Actor%20Object%20Reference)))

(event EventTick
  (params (DeltaSeconds :type Float%20%28single-precision%29))
  ;[1 1 1] Управление
  (CallFunction|MoviFlyEnter)
  ;[1 1 1] Луч управления ракетой
  (CallFunction|RayControlRocket)
  (CallFunction|DistanceBomb)
  (Transformation|SetWorldRotation (Variables|Default|GetStaticMesh1) (Transformation|GetActorRotation) false false)
  (Transformation|AddRelativeRotation (Variables|Default|GetStaticMesh2) "0, 0,30.000000" false false)
  (CallFunction|InvisibilityObject (> (.z (Transformation|GetWorldLocation (Variables|Default|GetStaticMesh1))) 2.51e+04))
  (CallFunction|FireRocket1)
  (CallFunction|FireRocket2))

(event Input|AxisEvents|InputAxisTurnRight/LeftMouse
  (params (AxisValue :type Float%20%28single-precision%29))
  ;[1 1 1] Обзор камеры по горизонтали
  (Transformation|SetRelativeRotation (Variables|Default|GetArrow) (Math|Rotator|MakeRotator 0.0 0.0 (Math|Float|Clamp(Float) (+ (.yaw (Variables|/Script/Engine.SceneComponent|GetRelativeRotation (Variables|Default|GetArrow))) (/ AxisValue 2.0)) -9e+01 9e+01)) false false))

(event Input|AxisEvents|InputAxisLookUp/DownMouse
  (params (AxisValue :type Float%20%28single-precision%29))
  (bind _cameravertical (Variables|Default|GetCameraVertical))
  (bind _relativerotation (Variables|/Script/Engine.SceneComponent|GetRelativeRotation _cameravertical))
  ;[1 1 1] Обзор камеры по вертикале
  (Transformation|SetRelativeRotation (Variables|Default|GetCameraVertical) (Math|Rotator|MakeRotator (.roll _relativerotation) (Math|Float|Clamp(Float) (- (.pitch _relativerotation) (/ AxisValue 2.0)) -25.0 25.0) (.yaw _relativerotation)) false false))

(event Input|KeyboardEvents|A
  (params (Key :type Key%20Structure :default "None"))
  ;[1 1 1] Поворот вправо и влево
  (:Pressed
    (Variables|Default|Setleft/Right -0.1))
  (:Released
    (Variables|Default|Setleft/Right 0.0)))

(event Input|KeyboardEvents|D
  (params (Key :type Key%20Structure :default "None"))
  ;[1 1 1] Поворот вправо и влево
  (:Pressed
    (Variables|Default|Setleft/Right 0.1))
  (:Released
    (Variables|Default|Setleft/Right 0.0)))

(event Input|KeyboardEvents|E
  (params (Key :type Key%20Structure :default "None"))
  ;[1 1 1] Выход из байрактара
  (:Pressed
    (bind _returnvalue (Game|SpawnActorfromClass "/Game/Kvik/Kvik_Modes/Players/Player_Hand/Test_hand/BP_Kv_PlayerHand_Pawn.BP_Kv_PlayerHand_Pawn_C" (Transformation|GetActorTransform (Variables|Default|GetSpawn_Player)) "Undefined" 0 0))
    (Pawn|Possess (Game|GetPlayerController 0) _returnvalue)
    (Viewport|RemoveAllWidgets)
    (bind _returnvalue_2 (UserInterface|CreateWidget "/Game/Kvik/Kv_UI_Canvas/UI_Kv_Intepface.UI_Kv_Intepface_C"))
    (UserInterface|Viewport|AddtoViewport _returnvalue_2 0)
    (CallFunction|LoadAmmo)
    (Variables|Default|Setleft/Right 0.1)))

(event Input|KeyboardEvents|LeftCtrl
  (params (Key :type Key%20Structure :default "None"))
  ;[1 1 1] Регулеровка высоты
  (:Pressed
    (Variables|Default|SetUp/Down -3.0))
  (:Released
    (Variables|Default|SetUp/Down 0.0)))

(event Input|KeyboardEvents|LeftAlt
  (params (Key :type Key%20Structure :default "None"))
  ;[1 1 1] Регулеровка высоты
  (:Pressed
    (Variables|Default|SetUp/Down 3.0))
  (:Released
    (Variables|Default|SetUp/Down 0.0)))

(event Input|MouseEvents|LeftMouseButton
  (params (Key :type Key%20Structure :default "None"))
  ;[1 1 1] Сброс боеприпаса
  (:Pressed
    (if (Variables|Default|Getmod_Fire)
      (if (> (Variables|Default|GetNumber_Bomb) 0)
        (switch int (Variables|Default|GetNumber_Bomb)
          (:1
            (Physics|SetSimulatePhysics (Variables|Default|GetSlot_Bomb_2) true))
          (:2
            (Physics|SetSimulatePhysics (Variables|Default|GetSlot_Bomb_1) true)))
        (Variables|Default|SetNumber_Bomb (- (Variables|Default|GetNumber_Bomb) 1)))
      (elif (> (Variables|Default|GetNumber_Rocket) 0)
        (if (Utilities|Operators|NotEqual(!=) :A (Variables|Default|GetTarget_Rocket))
          (switch int (Variables|Default|GetNumber_Rocket)
            (:1
              (Variables|Default|SetRocket_2_Fire true))
            (:2
              (Variables|Default|SetRocket_1_Fire true)))
          (Variables|Default|SetNumber_Rocket (- (Variables|Default|GetNumber_Rocket) 1))
          (else
            (Development|PrintString "Нет цели")))))))

(event Input|KeyboardEvents|1
  (params (Key :type Key%20Structure :default "None"))
  ;[1 1 1] Выбор типа боеприпаса
  (:Pressed
    (Variables|Default|Setmod_Fire false)))

(event Input|KeyboardEvents|2
  (params (Key :type Key%20Structure :default "None"))
  ;[1 1 1] Выбор типа боеприпаса
  (:Pressed
    (Variables|Default|Setmod_Fire true)))

(event Input|MouseEvents|MouseWheelUp
  (params (Key :type Key%20Structure :default "None"))
  ;[1 1 1] Приближение камеры
  (:Pressed
    (Camera|SetFieldOfView (Variables|Default|GetCamera) 4e+01)))

(event Input|MouseEvents|MouseWheelDown
  (params (Key :type Key%20Structure :default "None"))
  ;[1 1 1] Приближение камеры
  (:Pressed
    (Camera|SetFieldOfView (Variables|Default|GetCamera) 9e+01)))

(fn ConstructionScript)

(fn MoviFlyEnter
  (bind _defaultsceneroot (Variables|Default|GetDefaultSceneRoot))
  (bind _returnvalue (Math|Vector|GetForwardVector _defaultsceneroot))
  (bind _returnvalue_2 (* (Math|Vector|MakeVector (.x _returnvalue) (.y _returnvalue) 0.0) 5))
  (Transformation|AddRelativeRotation (Variables|Default|GetBayraktarTB2_Bayraktar) "0, 0,30.000000" false false)
  (Class|SceneComponent|AddWorldTransform _defaultsceneroot (Math|Transform|MakeTransform (Math|Vector|MakeVector (.x _returnvalue_2) (.y _returnvalue_2) (Variables|Default|GetUp/Down)) (Math|Rotator|MakeRotator 0.0 0.0 (Variables|Default|Getleft/Right)) "1.000000,1.000000,1.000000") false false))

(fn RayControlRocket
  (bind _camera (Variables|Default|GetCamera))
  (bind _returnvalue (Transformation|GetWorldLocation _camera))
  (bind _outhit (Class|KismetSystemLibrary|LineTraceSinglebyProfile (+ _returnvalue "0,0,-25.000000") (+ _returnvalue (* (Math|Vector|GetForwardVector _camera) 1e+05)) "None" false 0 "None" true))
  (if (.bBlockingHit (Collision|BreakHitResult _outhit))
    (bind _output_get (Variables|Default|SetTarget_Rocket (.ImpactPoint (Collision|BreakHitResult _outhit))))
    (return _output_get)
    (else
      (Variables|Default|SetTarget_Rocket "0, 0, 0"))))

(fn InvisibilityObject
  (params (Fun_invisibility :type Boolean))
  (if Fun_invisibility
    ;[1 1 1] Невидемость
    (bind _output_get (Variables|Default|Setparameter_Invision (Math|Interpolation|FInterptoConstant (Variables|Default|Getparameter_Invision) 0.0 (Utilities|Time|GetWorldDeltaSeconds) 0.1)))
    (Rendering|Material|SetScalarParameterValueonMaterials (Variables|Default|GetStaticMesh) "invisibility" _output_get)
    (else
      ;[1 1 1] Невидемость
      (bind _output_get_2 (Variables|Default|Setparameter_Invision (Math|Interpolation|FInterptoConstant (Variables|Default|Getparameter_Invision) 1.0 (Utilities|Time|GetWorldDeltaSeconds) 0.1)))
      (Rendering|Material|SetScalarParameterValueonMaterials (Variables|Default|GetStaticMesh) "invisibility" _output_get_2))))
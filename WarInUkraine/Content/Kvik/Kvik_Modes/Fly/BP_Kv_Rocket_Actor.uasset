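; BP_Kv_Rocket_Actor is a homing rocket for Kvik's Fly mode that explodes on overlap.
; Tick moves it along local X by KvSpeedRocket per frame, unscaled by delta time, while slowly interpolating rotation toward Target.
; Mesh overlap with any actor not tagged "Bayraktar" spawns BP_Kv_ExplosionBig and destroys the rocket.
; A Delay in Tick also destroys it after a fixed lifetime.
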(event OnComponentHit(StaticMesh)
  (params (HitComponent :type Primitive%20Component%20Object%20Reference) (OtherActor :type Actor%20Object%20Reference) (OtherComp :type Primitive%20Component%20Object%20Reference) (NormalImpulse :type Vector :default "0, 0, 0") (Hit :type Hit%20Result%20Structure%20%28by%20ref%29)))

(event OnComponentBeginOverlap(StaticMesh)
  (params (OverlappedComponent :type Primitive%20Component%20Object%20Reference) (OtherActor :type Actor%20Object%20Reference) (OtherComp :type Primitive%20Component%20Object%20Reference) (OtherBodyIndex :type Integer) (bFromSweep :type Boolean) (SweepResult :type Hit%20Result%20Structure%20%28by%20ref%29))
  (if (not (Actor|ActorHasTag OtherActor "Bayraktar"))
    (Game|SpawnActorfromClass "/Game/Kvik/Effects/BP_Kv_ExplosionBig.BP_Kv_ExplosionBig_C" (Transformation|GetActorTransform) "Undefined" 0 0)
    (Development|PrintString "2")
    (Actor|DestroyActor)))

(event EventBeginPlay)

(event Collision|EventActorBeginOverlap
  (params (OtherActor :type Actor%20Object%20Reference)))

(event EventTick
  (params (DeltaSeconds :type Float%20%28single-precision%29))
  (bind _returnvalue (Transformation|GetActorLocation))
  (bind _target (Variables|Default|GetTarget))
  (bind _returnvalue_2 (Math|Rotator|FindLookatRotation _returnvalue _target))
  (Class|SceneComponent|AddLocalTransform (Variables|Default|GetDefaultSceneRoot) (Math|Transform|MakeTransform (Math|Vector|MakeVector (Variables|Default|GetKv_Speed_Rocket) 0.0 0.0) "0.0,0.0,0.0" "1.000000,1.000000,1.000000") false false)
  (Transformation|SetActorRotation (Math|Interpolation|RInterpTo (Transformation|GetActorRotation) (Math|Rotator|MakeRotator (.roll _returnvalue_2) (.pitch _returnvalue_2) (.yaw _returnvalue_2)) (Utilities|Time|GetWorldDeltaSeconds) 0.5))
  (Utilities|FlowControl|Delay 3e+01)
  (Actor|DestroyActor))

(fn ConstructionScript)
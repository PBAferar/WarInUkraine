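; Stugna anti-tank missile launcher pawn with a remote laptop sight, guided rocket and self-adjusting legs.
; Tick turns and pitches the camera pivot within limits, lowers each leg value until its trigger overlaps, and prints delayed placement status.
; With the laptop open, a scene capture renders to texture and its forward trace feeds the rocket's target point.
; Firing requires installed and loaded states, shown by lights and tube material; a box flags Kv_BP_Man for reloading.
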(event OnComponentBeginOverlap(Box1)
  (params (OverlappedComponent :type Primitive%20Component%20Object%20Reference) (OtherActor :type Actor%20Object%20Reference) (OtherComp :type Primitive%20Component%20Object%20Reference) (OtherBodyIndex :type Integer) (bFromSweep :type Boolean) (SweepResult :type Hit%20Result%20Structure%20%28by%20ref%29))
  ;[0 1 0.06974] Триггеры лап
  (Variables|Default|SetB_Lap_1 false))

(event OnComponentBeginOverlap(Box3)
  (params (OverlappedComponent :type Primitive%20Component%20Object%20Reference) (OtherActor :type Actor%20Object%20Reference) (OtherComp :type Primitive%20Component%20Object%20Reference) (OtherBodyIndex :type Integer) (bFromSweep :type Boolean) (SweepResult :type Hit%20Result%20Structure%20%28by%20ref%29))
  ;[0 1 0.06974] Триггеры лап
  (Variables|Default|SetB_Lap_3 false))

(event OnComponentBeginOverlap(Box2)
  (params (OverlappedComponent :type Primitive%20Component%20Object%20Reference) (OtherActor :type Actor%20Object%20Reference) (OtherComp :type Primitive%20Component%20Object%20Reference) (OtherBodyIndex :type Integer) (bFromSweep :type Boolean) (SweepResult :type Hit%20Result%20Structure%20%28by%20ref%29))
  ;[0 1 0.06974] Триггеры лап
  (Variables|Default|SetB_Lap_2 false))

(event OnComponentBeginOverlap(BoxReload)
  (params (OverlappedComponent :type Primitive%20Component%20Object%20Reference) (OtherActor :type Actor%20Object%20Reference) (OtherComp :type Primitive%20Component%20Object%20Reference) (OtherBodyIndex :type Integer) (bFromSweep :type Boolean) (SweepResult :type Hit%20Result%20Structure%20%28by%20ref%29))
  ;[0 1 0.09189] Триггер презарядки
  (Utilities|Casting|CastToKv_BP_Man OtherActor)
  (Variables|Default|SetKv_PointReload true))

(event OnComponentEndOverlap(BoxReload)
  (params (OverlappedComponent :type Primitive%20Component%20Object%20Reference) (OtherActor :type Actor%20Object%20Reference) (OtherComp :type Primitive%20Component%20Object%20Reference) (OtherBodyIndex :type Integer))
  ;[0 1 0.09189] Триггер презарядки
  (Utilities|Casting|CastToKv_BP_Man OtherActor)
  (Variables|Default|SetKv_PointReload false))

(event Custom|Fire_Rocket
  ;[0.1074 1 0.01446] Пуск ракеты
  (if (Variables|Default|GetKv_Installed)
    (if (Variables|Default|GetKv_ChargedStugna)
      (bind _returnvalue (Game|SpawnActorfromClass "/Game/Kvik/Kvik_Modes/Weapons/Stugna/Kv_Rocket_Stagna.Kv_Rocket_Stagna_C" (Transformation|GetWorldTransform (Variables|Default|GetSpawn_Rocket)) "Undefined" 0 0))
      (Variables|Default|SetKv_Stugna_Rocket _returnvalue)
      (Variables|Default|SetKv_ChargedStugna false)
      (CallFunction|FireandReloadTubusTexture))))

(event Custom|Closed_Laptop
  ;[1 0.2588 0] Удаление текстуры на камеру
  (Variables|/Script/Engine.SceneCaptureComponent2D|SetTextureTarget (Variables|Default|GetSceneCaptureComponent2D) 0)
  (Variables|Default|SetKv_Activation_Laptop false))

(event Custom|UpDeteNext
  ;[0 1 0.3186] Управление камеры по горизонтале
  (CallFunction|UpDate)
  (Transformation|SetWorldRotation (Variables|Default|GetPointRot) (Math|Rotator|MakeRotator 0.0 0.0 (+ (.yaw (Transformation|GetWorldRotation (Variables|Default|GetPointRot))) (Variables|Default|GetKv_RotCameraHorizontal))) false false)
  (Variables|Default|SetKv_RotCameraHorizontal (Math|Float|Clamp(Float) (+ (Variables|Default|GetKv_RotCameraHorizontal) (Variables|Default|GetKv_SpeedHorizontal)) -9e+01 9e+01))
  (CallFunction|ControlCameraVertical)
  ;[0 1 0.09827] Управление ракетой
  (bind _askv_rocket_stagna (Utilities|Casting|CastToKv_Rocket_Stagna (Variables|Default|GetKv_Stugna_Rocket)))
  (if (!= (Variables|Default|GetKv_Stugna_Rocket) 0)
    (Utilities|IsValid _askv_rocket_stagna
      (:Is%20Valid
        (Variables|/Game/Kvik/Kvik_Modes/Weapons/Stugna/Kv_Rocket_Stagna.Kv_Rocket_Stagna_C|SetHip_Point_Stugna _askv_rocket_stagna (Variables|Default|GetKv_hit_point))))))

(event Custom|Open_Laptop
  ;[1 0.2568 0] Назначение текстуры рендера на камеру
  (Variables|/Script/Engine.SceneCaptureComponent2D|SetTextureTarget (Variables|Default|GetSceneCaptureComponent2D) "/Game/Kvik/Taxture/Image/Kv_TextureRenderTarget2D.Kv_TextureRenderTarget2D")
  (Variables|Default|SetKv_Activation_Laptop true))

(event Custom|Reload_Srugna
  ;[0.03398 1 0.2079] Перезарядка
  (Variables|Default|SetKv_ChargedStugna true)
  (CallFunction|FireandReloadTubusTexture))

(event Custom|Take_Laptop
  ;[0 1 0.09952] Взят или нет планшет (Лампочки)
  (if (Variables|Default|GetKv_Installed)
    (Variables|Default|SetKv_Installed false)
    (Rendering|SetVisibility (Variables|Default|GetLight_Red) true false)
    (Rendering|SetVisibility (Variables|Default|GetLight_Green) false false)
    (else
      (Variables|Default|SetKv_Installed true)
      (Rendering|SetVisibility (Variables|Default|GetLight_Red) false false)
      (Rendering|SetVisibility (Variables|Default|GetLight_Green) true false))))

(event Custom|Fire_And_Reload_TubusTexture
  ;[1 0.4158 0] текстура тубуса
  (if (Variables|Default|GetKv_ChargedStugna)
    (Rendering|Material|SetMaterial (Variables|Default|GetGun) 0 "/AnimationSharing/AnimSharingGreen.AnimSharingGreen")
    (else
      (Rendering|Material|SetMaterial (Variables|Default|GetGun) 0 "/Engine/EngineMeshes/BackgroundMaterial.BackgroundMaterial"))))

(event Custom|UpDate
  ;[0.128 1 0.2784] Поворт лап стугны
  (if (Variables|Default|GetB_Lap_1)
    (Variables|Default|SetLapa_1 (Math|Float|Clamp(Float) (- (Variables|Default|GetLapa_1) 1.0) -1e+01 45.0)))
  (if (Variables|Default|GetB_Lap_2)
    (Variables|Default|SetLapa_2 (Math|Float|Clamp(Float) (- (Variables|Default|GetLapa_2) 1.0) -1e+01 45.0)))
  (if (Variables|Default|GetB_Lap_3)
    (Variables|Default|SetLapa_3 (Math|Float|Clamp(Float) (- (Variables|Default|GetLapa_3) 1.0) -1e+01 45.0))))

(event Custom|ControlCameraVertical
  (bind _scenecapturecomponent2d (Variables|Default|GetSceneCaptureComponent2D))
  (bind _pointrot (Variables|Default|GetPointRot))
  (bind _returnvalue (Transformation|GetWorldLocation _scenecapturecomponent2d))
  (bind _returnvalue_2 (Transformation|GetWorldRotation _pointrot))
  ;[0.001142 1 0.2621] Управление камеры по вертикале
  (Transformation|SetWorldRotation (Variables|Default|GetPointRot) (Math|Rotator|MakeRotator 0.0 (- (.pitch _returnvalue_2) (Variables|Default|GetKv_RotCameraVertical)) (.yaw _returnvalue_2)) false false)
  (Variables|Default|SetKv_RotCameraVertical (Math|Float|Clamp(Float) (+ (Variables|Default|GetKv_RotCameraVertical) (Variables|Default|GetKv_SpeedVertical)) -45.0 15.0))
  ;[0 1 0.1546] RayCast (виртуальный луч)
  (if (Variables|Default|GetKv_Activation_Laptop)
    (bind _outhit (Collision|LineTraceByChannel _returnvalue (+ _returnvalue (* (Math|Vector|GetForwardVector _scenecapturecomponent2d) (Variables|Default|GetKv_RayDistance))) "TraceTypeQuery1" true 0 "None" true "(R=1.000000,G=0.000000,B=0.000000,A=1.000000)" "(R=0.000000,G=1.000000,B=0.000000,A=1.000000)" 1.0))
    (Variables|Default|SetKv_hit_point (.ImpactPoint (Collision|BreakHitResult _outhit)))))

(event Custom|Instal
  (Utilities|FlowControl|Delay 3.0)
  (if (or (or (Variables|Default|GetB_Lap_1) (Variables|Default|GetB_Lap_2)) (Variables|Default|GetB_Lap_3))
    (Development|PrintString "нельзя установить")
    (else
      (Development|PrintString "Установлено"))))

(event EventBeginPlay
  ;[0.1462 1 0.2468] Проверка заряжен или нет
  (CallFunction|FireandReloadTubusTexture))

(event EventTick
  (params (DeltaSeconds :type Float%20%28single-precision%29))
  (CallFunction|UpDate)
  (CallFunction|UpDeteNext)
  (CallFunction|Instal))

(event Collision|EventActorBeginOverlap
  (params (OtherActor :type Actor%20Object%20Reference)))

(fn ConstructionScript)